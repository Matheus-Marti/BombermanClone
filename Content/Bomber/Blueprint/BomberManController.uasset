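; Player controller for a local two-player Bomberman game, carrying separate movement and bomb inputs for each player.
; Inputs drive the Bomber at player index 0 or 1 along fixed world axes, also broadcasting axis values through movement dispatchers.
; It registers with GameModeBomber on BeginPlay.
; On possess it caches the Bomber and, per the GameInstance shared-screen flag, adds a split-screen widget or views the game mode's main camera.
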(event `InputAction|Bomba2`
  (params (Key :type "Key Structure"))
  (:`Pressed`
    (bind _asbomber (cast `/Game/Bomber/Blueprint/Bomber` (`GameplayStatics.GetPlayerCharacter` 1)))
    (`/Game/Bomber/Blueprint/Bomber.ColocarBomba2` _asbomber)))

(event `InputAxis|MoveRight2`
  (params (AxisValue :type "Float (single-precision)"))
  (bind _asbomber (cast `/Game/Bomber/Blueprint/Bomber` (`GameplayStatics.GetPlayerCharacter` 1)))
  (`Pawn.AddMovementInput` _asbomber (1.0 0.0 0.0) AxisValue false)
  (`self.moverfowardevent` AxisValue))

(event `InputAxis|MoveForward2`
  (params (AxisValue :type "Float (single-precision)"))
  (bind _asbomber (cast `/Game/Bomber/Blueprint/Bomber` (`GameplayStatics.GetPlayerCharacter` 1)))
  (`Pawn.AddMovementInput` _asbomber (0.0 1.0 0.0) AxisValue false)
  (`self.moverrightevent` AxisValue))

(event `InputAction|Bomba`
  (params (Key :type "Key Structure"))
  (:`Pressed`
    (bind _asbomber (cast `/Game/Bomber/Blueprint/Bomber` (`GameplayStatics.GetPlayerCharacter` 0)))
    (`/Game/Bomber/Blueprint/Bomber.ColocarBomba1` _asbomber)))

(event `InputAxis|MoveRight`
  (params (AxisValue :type "Float (single-precision)"))
  (bind _asbomber (cast `/Game/Bomber/Blueprint/Bomber` (`GameplayStatics.GetPlayerCharacter` 0)))
  (`Pawn.AddMovementInput` _asbomber (1.0 0.0 0.0) AxisValue false)
  (`self.moverfowardevent` AxisValue))

(event `InputAxis|MoveForward`
  (params (AxisValue :type "Float (single-precision)"))
  (bind _asbomber (cast `/Game/Bomber/Blueprint/Bomber` (`GameplayStatics.GetPlayerCharacter` 0)))
  (`Pawn.AddMovementInput` _asbomber (0.0 1.0 0.0) AxisValue false)
  (`self.moverrightevent` AxisValue))

(event `self.ReceiveBeginPlay`
  (bind _asgame_mode_bomber (cast `/Game/Bomber/Blueprint/GameModeBomber` (`GameplayStatics.GetGameMode`)))
  (bind _output_get (set `self.GM` _asgame_mode_bomber))
  (`/Game/Bomber/Blueprint/GameModeBomber.ReceberControlador` _output_get self))

(event `self.ReceivePossess`
  (params (PossessedPawn :type "Pawn Object Reference"))
  (`|ExecutionSequence`
    (:`then_0`
      (bind _asbomber (cast `/Game/Bomber/Blueprint/Bomber` PossessedPawn))
      (set `self.Bomberman` _asbomber))
    (:`then_1`
      (bind _asgame_instance (cast `/Game/Bomber/Blueprint/GameInstance` (`GameplayStatics.GetGameInstance`)))
      (if (not (`/Game/Bomber/Blueprint/GameInstance.telaCompartilhada` _asgame_instance))
        (bind _returnvalue (`|CreateWidget` "/Game/Bomber/Menu/Dividid.Dividid_C" self))
        (bind _output_get (set `self.WBPDividida` _returnvalue))
        (`UserWidget.AddToPlayerScreen` _output_get 0)
        (else
          (bind _gm (`self.GM`)
            (:`then`
              (`self.SetViewTargetWithBlend` (`/Game/Bomber/Blueprint/GameModeBomber.CameraPrincipal` _gm)))
            (:`else`)))))))

(event `self.ReceiveUnPossess`
  (params (UnpossessedPawn :type "Pawn Object Reference"))
  (set `self.Bomberman` null))

(fn `UserConstructionScript`)