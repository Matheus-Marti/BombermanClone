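; TorreBomba is a timed bomb actor for a Bomberman-style game that bursts in four directions.
; On BeginPlay it caches the player's Bomber character, then plays a timeline that animates the mesh's world scale as a fuse before death.
; When the timeline finishes, ExplosãoDirecional spawns an Explosao actor at AreaExplosao facing each positive and negative X and Y world axis, then destroys the bomb.
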(event `self.ReceiveBeginPlay`
  (bind _staticmesh (`self.StaticMesh`))
  (`|ExecutionSequence`
    (:`then_0`
      (bind _asbomber (cast `/Game/Bomber/Blueprint/Bomber` (`GameplayStatics.GetPlayerCharacter` 0)))
      (set `self.Bomberman` _asbomber))
    (:`then_1`
      (bind (_direction _tamanho_antes_da_morte) (`Timeline|Timelime_Explosao`)
        (:`Update`
          (`/Engine/EditorBlueprintResources/StandardMacros.IsValid` _staticmesh
            (:`Is Valid`
              (`SceneComponent.SetWorldScale3D` _staticmesh (`KismetMathLibrary.Conv_DoubleToVector` _tamanho_antes_da_morte)))))
        (:`Finished`
          (`self.ExplosãoDirecional`))))))

(fn `ExplosãoDirecional`
  (for _array_element (`|MakeArray` (1.0 0.0 0.0) (0.0 1.0 0.0) (-1.0 0.0 0.0) (0.0 -1.0 0.0) :!type "Vector Structure")
    (`|SpawnActorFromClass` "/Game/Bomber/Blueprint/Explosao.Explosao_C" (`KismetMathLibrary.MakeTransform` (`SceneComponent.K2_GetComponentLocation` (`self.areaExplosao`)) (`KismetMathLibrary.Conv_VectorToRotator` _array_element)) "Undefined" "OverrideRootScale" null null))
  (`self.K2_DestroyActor`))

(fn `UserConstructionScript`)