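; Bomberman-style player character that collects power-ups and places bombs, with a HUD chosen for shared or split screen.
; Capsule overlap with items applies fire, speed, extra-bomb or tower-bomb boosts by category.
; Tick re-applies an angled camera, updates a timer and box-traces ahead for obstacles.
; Two identical placement functions spawn Bomba or TorreBomba when unblocked and under TotalBomba, though the used count resets after each spawn.
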(event `self.CapsuleComponent.OnComponentBeginOverlap`
  (params (OverlappedComponent :type "PrimitiveComponent Object Reference") (OtherActor :type "Actor Object Reference") (OtherComp :type "PrimitiveComponent Object Reference") (OtherBodyIndex :type Integer) (bFromSweep :type Boolean) (SweepResult :type "HitResult Structure (by ref)"))
  (bind _itemmaster (`self.itemMaster`))
  (bind _itemmaster_2 (`self.itemMaster`))
  (bind _itemmaster_3 (`self.itemMaster`))
  (bind _itemmaster_4 (`self.itemMaster`))
  (bind _charactermovement (`self.CharacterMovement`))
  (bind _asbp_item_master (cast `/Game/Bomber/Itens/BP_itemMaster` OtherActor))
  (set `self.itemMaster` _asbp_item_master)
  (`GameplayStatics.PlaySoundAtLocation` "/Game/Bomber/Sons/MusicaItem_Cue.MusicaItem_Cue" (`SceneComponent.K2_GetComponentLocation` (`self.ColocarBomba`)) (struct) 1.0 1.0 0.0 null null null)
  (`self.ConjuntoItens`)
  (`|ExecutionSequence`
    (:`then_0`
      (switch `/Game/Bomber/Itens/Item` (`.categoria_7_4D19474240F6DCA9B25D1FA6F0274420` (break `/Game/Bomber/Itens/Booster` (`/Game/Bomber/Itens/BP_itemMaster.Itens` (`self.itemMaster`))))
        (:`NewEnumerator0`
          (bind _result (`/Engine/EditorBlueprintResources/StandardMacros.IncrementInt` (`self.fogoextra`))
            (:`  `
              (set `self.fogoextra` _result)
              (set `self.+Fogo` (* (`self.+Fogo`) 2.0))
              (`/Engine/EditorBlueprintResources/StandardMacros.IsValid` _itemmaster_4
                (:`Is Valid`
                  (`self.K2_DestroyActor` _itemmaster_4))))))
        (:`NewEnumerator1`
          (bind _result_2 (`/Engine/EditorBlueprintResources/StandardMacros.IncrementInt` (`self.velocidade`))
            (:`  `
              (set `self.velocidade` _result_2)
              (set `CharacterMovementComponent.MaxWalkSpeed` (+ (`CharacterMovementComponent.MaxWalkSpeed` _charactermovement) 200.0) _charactermovement)
              (`/Engine/EditorBlueprintResources/StandardMacros.IsValid` _itemmaster_2
                (:`Is Valid`
                  (`self.K2_DestroyActor` _itemmaster_2))))))
        (:`NewEnumerator2`
          (bind _result_3 (`/Engine/EditorBlueprintResources/StandardMacros.IncrementInt` (`self.bombaextra`))
            (:`  `
              (set `self.bombaextra` _result_3)
              (bind _result_4 (`/Engine/EditorBlueprintResources/StandardMacros.IncrementFloat` (`self.TotalBomba`))
                (:`  `
                  (bind _output_get (set `self.TotalBomba` _result_4))
                  (`KismetSystemLibrary.PrintString` (`KismetStringLibrary.Conv_DoubleToString` _output_get))
                  (`/Engine/EditorBlueprintResources/StandardMacros.IsValid` _itemmaster_3
                    (:`Is Valid`
                      (`self.K2_DestroyActor` _itemmaster_3))))))))
        (:`NewEnumerator4`
          (set `self.bombatorre` true)
          (`/Engine/EditorBlueprintResources/StandardMacros.IsValid` _itemmaster
            (:`Is Valid`
              (`self.K2_DestroyActor` _itemmaster))))))))

(event `self.ReceiveTick`
  (params (DeltaSeconds :type "Float (single-precision)"))
  (bind _returnvalue (`self.K2_GetActorLocation`))
  (bind _camera (`self.Camera`))
  (`|ExecutionSequence`
    (:`then_0`
      (`SceneComponent.K2_SetRelativeLocation` _camera (0.0 0.0 608.0) false false)
      (`SceneComponent.K2_SetWorldRotation` _camera (struct :`Pitch` -60.0 :`Yaw` -90.0) false false)
      (`KismetSystemLibrary.Delay` 1.0)
      (set `self.tempofinal` (`KismetMathLibrary.FTrunc` (- (`KismetMathLibrary.Conv_IntToDouble` (`self.tempofinal`)) DeltaSeconds))))
    (:`then_1`
      (bind (_outhit _returnvalue_2) (`KismetSystemLibrary.BoxTraceSingleForObjects` :`Start` _returnvalue :`End` (+ _returnvalue (* (`self.GetActorForwardVector`) 50.0)) :`HalfSize` (20.0 20.0 20.0) :`ObjectTypes` (`|MakeArray` "ObjectTypeQuery1" "ObjectTypeQuery1" "ObjectTypeQuery1" :!type "EObjectTypeQuery Enum") :`DrawDebugType` "ForOneFrame"))
      (set `self.podecolocarbomba` _returnvalue_2))))

(event `self.ReceiveBeginPlay`
  (bind _asgame_instance (cast `/Game/Bomber/Blueprint/GameInstance` (`GameplayStatics.GetGameInstance`)))
  (if (`/Game/Bomber/Blueprint/GameInstance.telaCompartilhada` _asgame_instance)
    (bind _returnvalue (`|CreateWidget` "/Game/Bomber/Menu/Compartilhada.Compartilhada_C" (`GameplayStatics.GetPlayerController` 0)))
    (`UserWidget.AddToViewport` _returnvalue 0)
    (else
      (bind _returnvalue_2 (`|CreateWidget` "/Game/Bomber/Menu/Dividid.Dividid_C" (`GameplayStatics.GetPlayerController` 0)))
      (`UserWidget.AddToPlayerScreen` _returnvalue_2 0))))

(fn `ColocarBomba1`
  (bind (_returnvalue_location _returnvalue_rotation _returnvalue_scale) (`KismetMathLibrary.BreakTransform` (`SceneComponent.K2_GetComponentToWorld` (`self.ColocarBomba`))))
  (if (not (`self.podecolocarbomba`))
    (if (< (`self.BombaUsada`) (`self.TotalBomba`))
      (bind _result (`/Engine/EditorBlueprintResources/StandardMacros.IncrementFloat` (`self.BombaUsada`))
        (:`  `
          (set `self.BombaUsada` _result)
          (if (`self.bombatorre`)
            (`|SpawnActorFromClass` "/Game/Bomber/Blueprint/TorreBomba.TorreBomba_C" (`KismetMathLibrary.MakeTransform` _returnvalue_location (struct) _returnvalue_scale) "AlwaysSpawn" "OverrideRootScale" null null)
            (set `self.BombaUsada` 0.0)
            (else
              (`|SpawnActorFromClass` "/Game/Bomber/Blueprint/Bomba.Bomba_C" (`KismetMathLibrary.MakeTransform` _returnvalue_location (struct) _returnvalue_scale) "AlwaysSpawn" "OverrideRootScale" null null)
              (set `self.BombaUsada` 0.0))))))))

(fn `ColocarBomba2`
  (bind (_returnvalue_location _returnvalue_rotation _returnvalue_scale) (`KismetMathLibrary.BreakTransform` (`SceneComponent.K2_GetComponentToWorld` (`self.ColocarBomba`))))
  (if (not (`self.podecolocarbomba`))
    (if (< (`self.BombaUsada`) (`self.TotalBomba`))
      (bind _result (`/Engine/EditorBlueprintResources/StandardMacros.IncrementFloat` (`self.BombaUsada`))
        (:`  `
          (set `self.BombaUsada` _result)
          (if (`self.bombatorre`)
            (`|SpawnActorFromClass` "/Game/Bomber/Blueprint/TorreBomba.TorreBomba_C" (`KismetMathLibrary.MakeTransform` _returnvalue_location (struct) _returnvalue_scale) "AlwaysSpawn" "OverrideRootScale" null null)
            (set `self.BombaUsada` 0.0)
            (else
              (`|SpawnActorFromClass` "/Game/Bomber/Blueprint/Bomba.Bomba_C" (`KismetMathLibrary.MakeTransform` _returnvalue_location (struct) _returnvalue_scale) "AlwaysSpawn" "OverrideRootScale" null null)
              (set `self.BombaUsada` 0.0))))))))

(fn `ConjuntoItens`
  (`KismetArrayLibrary.Array_Add` (`self.Boosters`) (`/Game/Bomber/Itens/BP_itemMaster.Itens` (`self.itemMaster`))))

(fn `pegarItem`
  (params (NewParam3 :type "/Game/Bomber/Itens/BP_itemMaster Object Reference"))
  (returns (ativar :type Boolean) (quantidade :type Integer) (categoria :type Byte))
  (set `self.itemMaster` NewParam3)
  (`self.ConjuntoItens`)
  (for _array_element (`self.Boosters`)
    _)
  (bind (_ativar _quatidade _categoria) (break `/Game/Bomber/Itens/Booster` _array_element))
  (return _ativar _quatidade _categoria))

(fn `UserConstructionScript`)