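; CopiaExplosiva is a movable copy owned by a Bomber, driven by that player's movement input.
; On BeginPlay it finds the owner's BomberManController and binds to its forward and right movement dispatchers.
; The handlers apply forced movement along world -X and -Y, scaled by the axis value and MultiplicarVelocidade.
; Despite the name, it holds no explosion logic; its Fogo self-assignment changes nothing and MoveForward is empty.
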(event `self.ReceiveBeginPlay`
  (`parent.ReceiveBeginPlay`)
  (bind _asbomber (cast `/Game/Bomber/Blueprint/Bomber` (`self.GetOwner`)))
  (set `/Game/Bomber/Blueprint/Bomber.+Fogo` (`/Game/Bomber/Blueprint/Bomber.+Fogo` _asbomber) _asbomber)
  (bind _asbomber_man_controller (cast `/Game/Bomber/Blueprint/BomberManController` (`self.GetController` _asbomber)))
  (bind _output_get (set `self.playerController` _asbomber_man_controller))
  (add `/Game/Bomber/Blueprint/BomberManController.moverfowardevent` _output_get (delegate `MoveForwardCopiaExplosiva`))
  (add `/Game/Bomber/Blueprint/BomberManController.moverrightevent` _output_get (delegate `MoveRightCopiaExplosiva`)))

(event `MoveForwardCopiaExplosiva`
  (params (axisValue :type "Float (double-precision)"))
  (`self.AddMovementInput` (-1.0 0.0 0.0) (* axisValue (`self.multiplicarVelocidade`)) true))

(event `MoveRightCopiaExplosiva`
  (params (axisValue :type "Float (double-precision)"))
  (`self.AddMovementInput` (0.0 -1.0 0.0) (* axisValue (`self.multiplicarVelocidade`)) true))

(fn `MoveForward`)

(fn `UserConstructionScript`
  (`parent.UserConstructionScript`))