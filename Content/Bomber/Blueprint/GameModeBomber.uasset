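; Game mode for the Bomber game that sets up local two-player play and handles death.
; BeginPlay creates a second player and reads the GameInstance's TelaCompartilhada flag to disable splitscreen and show a shared-screen widget.
; In shared mode, ReceberControlador and ReceberCamera point the second player's controller at the stored main camera, covering either registration order.
; Morte pauses the game and shows the death widget with a mouse cursor.
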(event `self.ReceiveBeginPlay`
  (`|ExecutionSequence`
    (:`then_0`
      (bind _asgame_instance (cast `/Game/Bomber/Blueprint/GameInstance` (`GameplayStatics.GetGameInstance`)))
      (bind _output_get (set `self.gameInstance` _asgame_instance))
      (bind _telacompartilhada (`/Game/Bomber/Blueprint/GameInstance.telaCompartilhada` _output_get))
      (`GameplayStatics.SetForceDisableSplitscreen` _telacompartilhada)
      (if _telacompartilhada
        (bind _returnvalue (`|CreateWidget` "/Game/Bomber/Menu/Compartilhada.Compartilhada_C"))
        (set `self.WBPCompartilhada` _returnvalue)
        (`UserWidget.AddToViewport` _returnvalue 0)))
    (:`then_1`
      (bind _returnvalue_2 (`GameplayStatics.CreatePlayer` 1))
      (bind _asbomber_man_controller (cast `/Game/Bomber/Blueprint/BomberManController` _returnvalue_2))
      (`self.ReceberControlador` _asbomber_man_controller))))

(event `self.ReceiveTick`
  (params (DeltaSeconds :type "Float (single-precision)")))

(fn `CameraPrincipal`
  (returns (CameraPrincipal :type "/Game/Bomber/Blueprint/Camera Object Reference"))
  (return (`self.camera`)))

(fn `Morte`
  (`GameplayStatics.SetGamePaused` true)
  (bind _returnvalue (`|CreateWidget` "/Game/Bomber/Menu/Morte.Morte_C" (`GameplayStatics.GetPlayerController` 0)))
  (bind _output_get (set `self.WBPMorte` _returnvalue))
  (`UserWidget.AddToViewport` _output_get 0)
  (set `PlayerController.bShowMouseCursor` true (`GameplayStatics.GetPlayerController` 0))
  (`/Game/Bomber/Menu/Morte.HudMorte` (`self.WBPMorte`)))

(fn `ReceberCamera`
  (params (Camera :type "/Game/Bomber/Blueprint/Camera Object Reference"))
  (bind _asgame_instance (cast `/Game/Bomber/Blueprint/GameInstance` (`GameplayStatics.GetGameInstance`)))
  (set `self.camera` Camera)
  (if (`/Game/Bomber/Blueprint/GameInstance.telaCompartilhada` _asgame_instance)
    (`PlayerController.SetViewTargetWithBlend` (`self.playerController`) (`self.camera`) 0.0 "VTBlend_Linear" 0.0 false)))

(fn `ReceberControlador`
  (params (`[0]` :type "/Game/Bomber/Blueprint/BomberManController Object Reference"))
  (bind _asgame_instance (cast `/Game/Bomber/Blueprint/GameInstance` (`GameplayStatics.GetGameInstance`)))
  (set `self.playerController` (`|MakeArray` `[0]`))
  (`|ExecutionSequence`
    (:`then_0`
      (if (`/Game/Bomber/Blueprint/GameInstance.telaCompartilhada` _asgame_instance)
        (bind _camera (`self.camera`)
          (:`then`
            (`PlayerController.SetViewTargetWithBlend` (`self.playerController`) _camera 0.0 "VTBlend_Linear" 0.0 false))
          (:`else`))))))

(fn `UserConstructionScript`)